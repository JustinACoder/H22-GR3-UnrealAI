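; Test Blueprint with a first-person camera that prototypes Hangman word selection and guess matching, using debug prints.
; N toggles IsLoading; while true, every Tick reloads wordlist.txt, picks a random word and appends asterisks to the blank string.
; Characters matching Guess are set on a temporary array, leaving the printed blank string unchanged.
; Right mouse sets IsDrawing, but the line-trace UV drawing onto BP_AI's whiteboard is disconnected.
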(event `Key|RightMouseButton`
  (params (Key :type "Key Structure"))
  (:`Pressed`
    (set `self.isDrawing` true))
  (:`Released`
    (set `self.isDrawing` false)))

(event `self.ReceiveTick`
  (params (DeltaSeconds :type "Float (single-precision)"))
  (bind _currentword (`self.CurrentWord`))
  (bind _currentwordblank (`self.CurrentWordBlank`))
  (bind _guess (`self.Guess`))
  (bind _returnvalue (`KismetStringLibrary.Len` _currentword))
  (if (`self.isLoading`)
    (bind _returnvalue_2 (`CustomBlueprintHelper.LoadFileToString` "wordlist.txt"))
    (set `self.CurrentWord` (`|GetArrayItem` (`KismetStringLibrary.ParseIntoArray` _returnvalue_2 " \n" false) (`KismetMathLibrary.RandomInteger` 99)))
    (`KismetSystemLibrary.PrintString` _currentword true true (struct :`G` 0.66 :`B` 1.0 :`A` 1.0) 99.0)
    (`KismetSystemLibrary.PrintString` (`KismetStringLibrary.Conv_IntToString` _returnvalue))
    (for _ (range _returnvalue)
      (bind _output_get (set `self.CurrentWordBlank` (`KismetStringLibrary.Concat_StrStr` (stale _output_get) "*"))))
    (`KismetSystemLibrary.PrintString` (`self.CurrentWordBlank`) true true (struct :`G` 0.66 :`B` 1.0 :`A` 1.0) 99.0)
    (for (_array_element _array_index) (`KismetStringLibrary.GetCharacterArrayFromString` _currentword)
      (if (`KismetStringLibrary.EqualEqual_StrStr` _array_element _guess)
        (`KismetArrayLibrary.Array_Set` (`KismetStringLibrary.GetCharacterArrayFromString` _currentwordblank) _array_index _guess)
        (`KismetSystemLibrary.PrintString` _currentwordblank)))))

(event `Key|N`
  (params (Key :type "Key Structure"))
  (:`Pressed`
    (if (`self.isLoading`)
      (set `self.isLoading` false)
      (else
        (set `self.isLoading` true)))))

(fn `UserConstructionScript`)