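; Whiteboard actor that lets the player draw into a render target and classifies the drawing through an ML component running the emnist_loader script.
; DrawToWhiteboard stamps a dynamic marker material onto the render target at the drawn location.
; Key 0 converts the render target to a float array and sends it to the script, and key C clears the board.
; The result callback prints the index of the highest score as the prediction.
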(event `self.ReceiveBeginPlay`
  (bind _returnvalue (`KismetMaterialLibrary.CreateDynamicMaterialInstance` "/Game/UnrealAI_BP/M_WBMarker.M_WBMarker"))
  (set `self.MI_Marker` _returnvalue)
  (`KismetRenderingLibrary.ClearRenderTarget2D` "/Game/UnrealAI_BP/RT_InputAI.RT_InputAI")
  (`self.EnableInput` (`GameplayStatics.GetPlayerController` 0))
  (`MachineLearningRemoteComponent.StartScript` (`self.MLComponent`) "emnist_loader")
  (add `MachineLearningBaseComponent.OnRawInputResult` (`self.MLComponent`) (delegate `ML_Output`)))

(event `ML_Output`
  (params (ResultData :type "Array of Float (double-precision) (by ref)") (CallingFunctionName :type String))
  (`KismetSystemLibrary.PrintString` (`KismetStringLibrary.Conv_IntToString` (`KismetMathLibrary.MaxOfFloatArray` ResultData))))

(event `Key|Zero`
  (params (Key :type "Key Structure"))
  (:`Pressed`
    (`MachineLearningBaseComponent.SendRawInput` (`self.MLComponent`) (`TensorFlowBlueprintLibrary.Conv_GreyScaleTexture2DToFloatArray` (`TensorFlowBlueprintLibrary.Conv_RenderTargetTextureToTexture2D` "/Game/UnrealAI_BP/RT_InputAI.RT_InputAI")) "on_json_input")))

(event `Key|C`
  (params (Key :type "Key Structure"))
  (:`Pressed`
    (`KismetRenderingLibrary.ClearRenderTarget2D` "/Game/UnrealAI_BP/RT_InputAI.RT_InputAI")))

(event `Draw To Whiteboard`
  (params (`Drawn Location` :type "Vector2D Structure"))
  (bind _mi_marker (`self.MI_Marker`))
  (`MaterialInstanceDynamic.SetVectorParameterValue` _mi_marker "DrawLocation" (`KismetMathLibrary.Conv_VectorToLinearColor` (`KismetMathLibrary.Conv_Vector2DToVector` `Drawn Location`)))
  (`KismetRenderingLibrary.DrawMaterialToRenderTarget` "/Game/UnrealAI_BP/RT_InputAI.RT_InputAI" _mi_marker))

(fn `UserConstructionScript`)