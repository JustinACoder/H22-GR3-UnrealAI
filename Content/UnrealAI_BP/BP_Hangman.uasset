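; BP_Hangman runs a hangman word-guessing minigame, creating its WBP_Hangman widget at BeginPlay and toggling visibility through open and close events.
; A randomly indexed word from GetHangManWord becomes an underscore mask, which guesses fill by substring search and character-array replacement.
; Wrong or already-revealed letters increment the error count.
; A separate check event counts solved words and resets letters and errors, without drawing a new word.
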(event `Check word`
  ;[1 1 1] Check if the shown word is the same as the real word
  (if (`KismetStringLibrary.EqualEqual_StrStr` (`self.Word to find`) (`self.Word to show`))
    (`/Engine/EditorBlueprintResources/StandardMacros.IncrementInt` (`self.Word found`)
      (:`  `
        (set `self.Letters used` "")
        (set `self.Errors` 0)))))

(event `self.ReceiveBeginPlay`
  ;[1 1 1] Create the hang man game with the interface hidden
  (bind _returnvalue (`|CreateWidget` "/Game/UnrealAI_BP/WBP_Hangman.WBP_Hangman_C"))
  (bind _output_get (set `self.HG_Interface` _returnvalue))
  (`UserWidget.AddToViewport` _output_get 0)
  (`self.Get Word to Find`)
  (`self.Close HangMan Game`))

(event `Open HangMan Game`
  ;[1 1 1] Make the hang man game visible
  (`Widget.SetVisibility` (`self.HG_Interface`) "Visible"))

(event `Close HangMan Game`
  ;[1 1 1] Make the hang man game invisible
  (`Widget.SetVisibility` (`self.HG_Interface`) "Collapsed"))

(event `Get Word to Find`
  ;[1 1 1] Get a word in the list to use in the game
  (bind _returnvalue (`CustomBlueprintHelper.getHangManWord` (`KismetMathLibrary.RandomInteger` 100)))
  (bind _output_get (set `self.Word to find` _returnvalue))
  (set `self.Word to show` "")
  (for _ (range (+ (`KismetStringLibrary.Len` _output_get) 1))
    (set `self.Word to show` (`KismetStringLibrary.Concat_StrStr` (`self.Word to show`) "_"))))

(event `Replace in word to show`
  (params (Letter :type String))
  (bind _returnvalue (`KismetStringLibrary.ParseIntoArray` (`self.Word to show`)))
  ;[1 1 1] Replace the right letters in the word to show
  (for _ (range (+ (`KismetStringLibrary.Len` (`self.Word to find`)) 1))
    (bind _output_get (set `self.Letter position` (`KismetStringLibrary.FindSubstring` (`self.Word to find`) Letter false false (`self.Letter position`))))
    (`KismetArrayLibrary.Array_Set` _returnvalue _output_get Letter)
    (set `self.Word to show` (`KismetStringLibrary.JoinStringArray` _returnvalue)))
  (set `self.Letter position` 0))

(event `Make a guess`
  (params (Letter :type String))
  ;[1 1 1] Take a guess from the user
  (set `self.Letters used` (`KismetStringLibrary.Concat_StrStr` (`self.Letters used`) Letter))
  (if (and (`KismetStringLibrary.Contains` (`self.Word to find`) Letter) (not (`KismetStringLibrary.Contains` (`self.Word to show`) Letter)))
    (`self.Replace in word to show` Letter)
    (else
      (`/Engine/EditorBlueprintResources/StandardMacros.IncrementInt` (`self.Errors`)))))