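; BP_QuickDraw is a controller Blueprint for a Quick, Draw-style drawing game in which the player is given a word to draw.
; On BeginPlay it creates the WBP_QuickDraw widget, picks a word and hides the interface, with events to open and close it.
; Words come from GetQuickDrawLabel using a random label index and are passed to the widget.
; CheckWord compares an incoming prediction to the current word and picks a new one on a match.
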(event `self.ReceiveBeginPlay`
  ;[1 1 1] Create the actor with the interface hidden
  (bind _returnvalue (`|CreateWidget` "/Game/UnrealAI_BP/WBP_QuickDraw.WBP_QuickDraw_C"))
  (bind _output_get (set `self.Interface` _returnvalue))
  (`UserWidget.AddToViewport` _output_get 0)
  (`self.Get Word to Draw`)
  (`self.Close QuickDraw Game`))

(event `Open QuickDraw Game`
  ;[1 1 1] Start the game by making the interface visible
  (`Widget.SetVisibility` (`self.Interface`) "Visible"))

(event `Close QuickDraw Game`
  ;[1 1 1] Start the game by making the interface visible
  (`Widget.SetVisibility` (`self.Interface`) "Collapsed"))

(event `Get Word to Draw`
  ;[1 1 1] Get the word to draw
  (bind _returnvalue (`CustomBlueprintHelper.getQuickDrawLabel` (`KismetMathLibrary.RandomInteger` 345) 100.0))
  (bind _output_get (set `self.Word to Draw` _returnvalue))
  (set `/Game/UnrealAI_BP/WBP_QuickDraw.CurrentWord` _output_get (`self.Interface`)))

(event `Check Word`
  (params (Prediction :type String))
  ;[1 1 1] Check if the word drawn is valid
  (if (`KismetStringLibrary.EqualEqual_StrStr` Prediction (`self.Word to Draw`))
    (`self.Get Word to Draw`)))

(fn `UserConstructionScript`)