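; Whiteboard Blueprint that records drawing strokes and submits a whiteboard image to an AI through a TensorFlow component.
; DrawOnWhiteboard feeds a location into a dynamic marker material and draws it onto a render target, which is cleared at BeginPlay.
; Pressing V imports WhiteboardOutput.exr from the project directory and sends it as JSON texture input, noted as slow above 512x512.
; The V handler appears twice, and no render target export happens here.
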(event `self.ReceiveBeginPlay`
  (bind _returnvalue (`KismetMaterialLibrary.CreateDynamicMaterialInstance` "/Game/Whiteboard/M_WhiteboardMarker.M_WhiteboardMarker"))
  (set `self.WhiteboardMarker_MI` _returnvalue)
  (`KismetRenderingLibrary.ClearRenderTarget2D` "/Game/Whiteboard/RT_Whiteboard.RT_Whiteboard")
  (`self.EnableInput` (`GameplayStatics.GetPlayerController` 0)))

(event `Draw On Whiteboard`
  (params (`Location To Draw` :type "Vector2D Structure"))
  (bind _whiteboardmarker_mi (`self.WhiteboardMarker_MI`))
  (`MaterialInstanceDynamic.SetVectorParameterValue` _whiteboardmarker_mi "DrawLocation" (`KismetMathLibrary.Conv_VectorToLinearColor` (`KismetMathLibrary.Conv_Vector2DToVector` `Location To Draw`)))
  (`KismetRenderingLibrary.DrawMaterialToRenderTarget` "/Game/Whiteboard/RT_Whiteboard.RT_Whiteboard" _whiteboardmarker_mi))

(event `Key|V`
  (params (Key :type "Key Structure"))
  ;[1 1 1] New section: Send the image on the whiteboard to the AI
  (:`Pressed`
    (bind _returnvalue (`KismetRenderingLibrary.ImportFileAsTexture2D` (`KismetStringLibrary.Concat_StrStr` (`KismetSystemLibrary.GetProjectDirectory`) "WhiteboardOutput.exr")))
    ;;[1 1 1] Really slow for textures bigger 512x512
    (`/TensorFlow/TensorflowComponent.SendJsonInputTexture` (`self.TensorflowComponent`) _returnvalue false false)))

(event `Key|V`
  (params (Key :type "Key Structure"))
  ;[1 1 1] New section: By pressing V, get the white board input and sends it to the AI
  (:`Pressed`
    (bind _returnvalue (`KismetRenderingLibrary.ImportFileAsTexture2D` (`KismetStringLibrary.Concat_StrStr` (`KismetSystemLibrary.GetProjectDirectory`) "WhiteboardOutput.exr")))
    (`/TensorFlow/TensorflowComponent.SendJsonInputTexture` (`self.TensorflowComponent`) _returnvalue false false)))

(fn `UserConstructionScript`)